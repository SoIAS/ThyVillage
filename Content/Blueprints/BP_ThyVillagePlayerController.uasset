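; Player controller that owns the player's inventory screen and interaction tooltip UI.
; On BeginPlay it registers the ThirdPersonCharacter's inventory with InventoryManager and creates a hidden BP_Inventory widget, which toggle, open and close events show or hide, refreshing it when shown.
; A tooltip event lazily creates a widget displaying the interactable object's name.
; Temporary R and Q debug keys add test items, and CreateInventoryWidget is an uncalled, unfinished stub.
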(event `self.ReceiveBeginPlay`
  ;[1 1 1] Begin Play
  (`self.SetupPlayerInventory`)
  (`ThyVillageInventoryManager.SetStorageInventory` (`self.InventoryManager`) null)
  (`self.tmpstorage`))

(event `InputAction|ToggleInventory`
  (params (Key :type "Key Structure"))
  ;[1 1 1] Toggle Inventory Input
  (:`Pressed`
    (`self.ToggleInventory`)
    (set `self.bShowMouseCursor` (`Widget.IsVisible` (`self.InventoryWidget`)))))

(event `self.ToggleInventory`
  (bind _inventorywidget (`self.InventoryWidget`))
  ;[1 1 1] Toggles Inventory implementation (creates one if it is not valid)
  (if (not (`KismetSystemLibrary.IsValid` _inventorywidget))
    (`self.tmpstorage`))
  (if (`Widget.IsVisible` _inventorywidget)
    (`Widget.SetVisibility` _inventorywidget "Hidden")
    (else
      (`Widget.SetVisibility` _inventorywidget "Visible")
      (`self.updateinv`)
      (set `self.bShowMouseCursor` true))))

(event `self.OpenInventory`
  ;[1 1 1] Show inventory implementation
  (if (not (`KismetSystemLibrary.IsValid` (`self.InventoryWidget`)))
    (`self.tmpstorage`))
  (`Widget.SetVisibility` (`self.InventoryWidget`) "Visible")
  (`self.updateinv`)
  (set `self.bShowMouseCursor` true))

(event `self.CloseInventory`
  ;[1 1 1] Hide inventory implementation
  (if (`KismetSystemLibrary.IsValid` (`self.InventoryWidget`))
    (`Widget.SetVisibility` (`self.InventoryWidget`) "Hidden")
    (set `self.bShowMouseCursor` false)))

(event `Key|R`
  (params (Key :type "Key Structure"))
  ;[1 1 1] Temp itema dding removeing
  (:`Pressed`
    (bind _asthird_person_character (cast `/Game/ThirdPersonCPP/Blueprints/ThirdPersonCharacter` (`self.K2_GetPawn`)))
    (bind _thevillageinventory (`/Game/ThirdPersonCPP/Blueprints/ThirdPersonCharacter.TheVillageInventory` _asthird_person_character))
    (`TheVillageInventoryComponent.AddItemExact` _thevillageinventory "/Game/Items/Resources/Metal.Metal" 7)
    (`TheVillageInventoryComponent.AddItemExact` _thevillageinventory "/Game/Items/Resources/Wood.Wood" 6)
    (`self.updateinv` :!label _label)))

(event `self.OnInteractionTooltip`
  (params (bShow :type Boolean) (InteractableObjet :type "ThyVillageInteractableActor Object Reference"))
  (if (and bShow (`KismetSystemLibrary.IsValid` InteractableObjet))
    (`self.ShowInteractionTooltip`)
    (`/Game/Blueprints/Widgets/Interaction/BP_InteractionTooltip.SetInteractionTooltip` (`self.InteractionTooltip`) (`ThyVillageInteractableActor.InteractableName` InteractableObjet))
    (else
      (`self.HideInteractionTooltip`))))

(event `Key|Q`
  (params (Key :type "Key Structure"))
  ;[1 1 1] Temp itema dding removeing
  (:`Pressed`
    (bind _asthird_person_character (cast `/Game/ThirdPersonCPP/Blueprints/ThirdPersonCharacter` (`self.K2_GetPawn`)))
    (bind _thevillageinventory (`/Game/ThirdPersonCPP/Blueprints/ThirdPersonCharacter.TheVillageInventory` _asthird_person_character))
    (`TheVillageInventoryComponent.AddItemExact` _thevillageinventory "/Game/Items/Resources/Sulphir.Sulphir" 4)
    (`TheVillageInventoryComponent.AddItemExact` _thevillageinventory "/Game/Items/Resources/Water.Water" 11)
    (goto _label)))

(fn `CreateInteractionTooltipWidget`
  (bind _returnvalue (`|CreateWidget` "/Game/Blueprints/Widgets/Interaction/BP_InteractionTooltip.BP_InteractionTooltip_C" self))
  (bind _output_get (set `self.InteractionTooltip` _returnvalue))
  (`UserWidget.AddToViewport` _output_get 0)
  (`Widget.SetVisibility` _output_get "Hidden"))

(fn `CreateInventoryWidget`
  (`|CreateWidget` "/Game/Blueprints/Widgets/Inventory/BP_InventoryGrid.BP_InventoryGrid_C" self))

(fn `HideInteractionTooltip`
  (bind _interactiontooltip (`self.InteractionTooltip`))
  (if (`KismetSystemLibrary.IsValid` _interactiontooltip)
    (`Widget.SetVisibility` _interactiontooltip "Hidden")))

(fn `SetupPlayerInventory`
  (bind _asthird_person_character (cast `/Game/ThirdPersonCPP/Blueprints/ThirdPersonCharacter` (`self.K2_GetPawn`))
    (:`then`
      (`ThyVillageInventoryManager.SetPlayerInventory` (`self.InventoryManager`) (`/Game/ThirdPersonCPP/Blueprints/ThirdPersonCharacter.TheVillageInventory` _asthird_person_character)))
    (:`CastFailed`
      (`KismetSystemLibrary.PrintString` "Cannot cast to Pawn"))))

(fn `ShowInteractionTooltip`
  (if (not (`KismetSystemLibrary.IsValid` (`self.InteractionTooltip`)))
    (`self.CreateInteractionTooltipWidget`))
  (`Widget.SetVisibility` (`self.InteractionTooltip`) "Visible"))

(fn `tmpstorage`
  (bind _returnvalue (`|CreateWidget` "/Game/Blueprints/Widgets/Inventory/BP_Inventory.BP_Inventory_C" self))
  (bind _output_get (set `self.InventoryWidget` _returnvalue))
  (`UserWidget.AddToViewport` _returnvalue 0)
  (`Widget.SetVisibility` _output_get "Hidden"))

(fn `updateinv`
  (`/Game/Blueprints/Widgets/Inventory/BP_Inventory.temp updated` (`self.InventoryWidget`)))

(fn `UserConstructionScript`)